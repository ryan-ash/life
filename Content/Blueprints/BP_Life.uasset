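; BP_Life runs a Life-style cellular simulation and shows it on an in-world screen.
; On BeginPlay it flattens InitialNodes patterns, offset by their roots, into a row-to-columns map of starting live cells, then calls Initialize.
; A dynamic material on the screen's display receives the simulation texture as a parameter.
; ChangeSpeed steps through preset delays, updates LifeHUD and restarts the looping LifeIteration timer, with zero delay pausing it.
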(event `self.ReceiveBeginPlay`
  (`self.Init`)
  (`self.PrepareTexture`))

(fn `ChangeSpeed`
  (params (RaiseSpeed :type Boolean))
  (bind _selecteddelay (`self.SelectedDelay`))
  (bind _returnvalue (- (`KismetArrayLibrary.Array_Length` (`self.Delays`)) 1))
  (bind _output_get (set `self.SelectedDelayID` (`KismetMathLibrary.Clamp` (+ (`self.SelectedDelayID`) (select `bool` RaiseSpeed :`false` -1 :`true` 1)) 0 _returnvalue)))
  (set `self.SelectedDelay` (`|GetArrayItem` (`self.Delays`) _output_get))
  (`/Game/Blueprints/UI/LifeHUD.SetLifeSpeed` (cast `/Game/Blueprints/UI/LifeHUD` (`PlayerController.GetHUD` (`GameplayStatics.GetPlayerController` 0)) :!pure true) (`self.SelectedDelayID`) _returnvalue)
  (`KismetSystemLibrary.K2_ClearAndInvalidateTimerHandle` (`self.IterationTimer`))
  (if (not (== _selecteddelay 0.0))
    (bind _returnvalue_2 (`KismetSystemLibrary.K2_SetTimer` null "LifeIteration" _selecteddelay true))
    (set `self.IterationTimer` _returnvalue_2)))

(fn `Init`
  (`self.PrepareInitialNodesCache`)
  (`self.Initialize`))

(fn `PrepareInitialNodesCache`
  (locals (RowBeingCached :type Integer) (ColumnBeingCached :type Integer) (Cells :type "Array of Integer"))
  (bind _cellsaliveatstart (`self.CellsAliveAtStart`))
  (bind _rowbeingcached (`local.RowBeingCached`))
  (bind _value (`BlueprintMapLibrary.Map_Find` _cellsaliveatstart _rowbeingcached))
  (`BlueprintMapLibrary.Map_Clear` (`self.CellsAliveAtStart`))
  (for _array_element (`self.InitialNodes`)
    (bind (_name _cells _rootoffset) (break `/Game/Types/Structs/LifeShape` _array_element))
    (for _array_element_2 _cells
      (bind (_row _column) (break `/Game/Types/Structs/LifeCell` _rootoffset))
      (bind (_row_2 _column_2) (break `/Game/Types/Structs/LifeCell` _array_element_2))
      (set `local.RowBeingCached` (+ _row _row_2))
      (set `local.ColumnBeingCached` (+ _column_2 _column))
      (if (`BlueprintMapLibrary.Map_Contains` _cellsaliveatstart _rowbeingcached)
        (bind _output_get (set `local.Cells` (`.Cells` (break `CellBlock` _value))))
        (`KismetArrayLibrary.Array_Add` _output_get (`local.ColumnBeingCached`))
        (bind _structout (setmembers `CellBlock` :`StructRef` _value :`Cells` (`local.Cells`)))
        (`BlueprintMapLibrary.Map_Add` (`self.CellsAliveAtStart`) (`local.RowBeingCached`) _structout)
        (else
          (`BlueprintMapLibrary.Map_Add` _cellsaliveatstart _rowbeingcached (make `CellBlock` (`|MakeArray` (`local.ColumnBeingCached`)))))))))

(fn `PrepareTexture`
  (bind _display (`/Game/Blueprints/SimpleScreen.Display` (`self.Screen`)))
  (bind _returnvalue (`PrimitiveComponent.CreateDynamicMaterialInstance` _display 0 "/Game/Materials/LifeMaterial.LifeMaterial" "None"))
  (bind _output_get (set `self.ScreenMaterial` _returnvalue))
  (`PrimitiveComponent.SetMaterial` _display 0 _output_get)
  (`DynamicTexture.UpdateTexture` (`self.Texture`))
  (`self.UpdateScreen`))

(fn `UpdateScreen`
  (`MaterialInstanceDynamic.SetTextureParameterValue` (`self.ScreenMaterial`) "Texture" (`DynamicTexture.GetTextureResource` (`self.Texture`))))

(fn `UserConstructionScript`)