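; Conway's Game of Life Blueprint that seeds a bounded cell grid from offset shapes cached by row at BeginPlay.
; A looping timer builds each new generation in a separate row buffer, with neighbour counts clamped at the edges.
; UpdateScreen paints cells white or black into a padded, nearest-filtered dynamic texture on the screen's material instance.
; In this graph it is called only during texture setup, not after each iteration.
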(event `self.ReceiveBeginPlay`
  (`self.Init`)
  (`self.PrepareTexture`)
  (`KismetSystemLibrary.K2_SetTimerDelegate` (delegate `Iterate`) 1.0 true))

(event `Iterate`
  (`self.LifeIteration`))

(fn `GetAliveNeighbours`
  (params (Row :type Integer) (Column :type Integer))
  (returns (AliveN :type Integer))
  (locals (CurrentAliveN :type Integer))
  (set `local.CurrentAliveN` 0)
  (for _index (range (`KismetMathLibrary.Max` (- Row 1)) (+ (`KismetMathLibrary.Min` (+ Row 1) (- (`self.Height`) 1)) 1))
    (for _index_2 (range (`KismetMathLibrary.Max` (- Column 1)) (+ (`KismetMathLibrary.Min` (+ Column 1) (- (`self.Width`) 1)) 1))
      (if (and (== _index (`local.Row`)) (== _index_2 (`local.Column`)))
        _
        (elif (`self.IsAlive` _index _index_2)
          (`/Engine/EditorBlueprintResources/StandardMacros.IncrementInt` (`local.CurrentAliveN`))))))
  (return (`local.CurrentAliveN`)))

(fn `Init`
  (locals (CurrentRow :type "/Game/Types/Structs/LifeRow Structure"))
  (`self.PrepareInitialNodesCache`)
  (`KismetArrayLibrary.Array_Clear` (`self.Rows`))
  (for _index (range (`self.Height`))
    (set `local.CurrentRow` (make `/Game/Types/Structs/LifeRow` _))
    (for _index_2 (range (`self.Width`))
      (bind (_value _returnvalue) (`BlueprintMapLibrary.Map_Find` (`self.CellsAliveAtStart`) _index))
      (`KismetArrayLibrary.Array_Add` (`.Cells_2_D70D34C248750123A4A2D180AB2CE047` (break `/Game/Types/Structs/LifeRow` (`local.CurrentRow`))) (and _returnvalue (`KismetArrayLibrary.Array_Contains` (`.Cells_3_2736CB634A50A057C35302ADDD968B86` (break `/Game/Types/Structs/LifeShapeRow` _value)) _index_2))))
    (`KismetArrayLibrary.Array_Add` (`self.Rows`) (`local.CurrentRow`))))

(fn `IsAlive`
  (params (Row :type Integer) (Column :type Integer))
  (returns (Alive :type Boolean))
  (return (`|GetArrayItem` (`.Cells_2_D70D34C248750123A4A2D180AB2CE047` (break `/Game/Types/Structs/LifeRow` (`|GetArrayItem` (`self.Rows`) Row))) Column)))

(fn `LifeIteration`
  (locals (CurrentRow :type "/Game/Types/Structs/LifeRow Structure") (NewRows :type "Array of /Game/Types/Structs/LifeRow Structure"))
  (`KismetArrayLibrary.Array_Clear` (`local.NewRows`))
  (`|ExecutionSequence`
    (:`then_0`
      (for _index (range (`self.Height`))
        (set `local.CurrentRow` (make `/Game/Types/Structs/LifeRow` _))
        (for _index_2 (range (`self.Width`))
          (bind _aliven (`self.GetAliveNeighbours` _index _index_2))
          (if (`self.IsAlive` _index _index_2)
            (`KismetArrayLibrary.Array_Add` (`.Cells_2_D70D34C248750123A4A2D180AB2CE047` (break `/Game/Types/Structs/LifeRow` (`local.CurrentRow`))) (`KismetMathLibrary.InRange_IntInt` _aliven 2 3))
            (else
              (`KismetArrayLibrary.Array_Add` (`.Cells_2_D70D34C248750123A4A2D180AB2CE047` (break `/Game/Types/Structs/LifeRow` (`local.CurrentRow`))) (== _aliven 3)))))
        (`KismetArrayLibrary.Array_Add` (`local.NewRows`) (`local.CurrentRow`)))
      (set `self.Rows` (`local.NewRows`)))))

(fn `PrepareInitialNodesCache`
  (locals (RowBeingCached :type Integer) (ColumnBeingCached :type Integer) (Cells :type "Array of Integer"))
  (bind _cellsaliveatstart (`self.CellsAliveAtStart`))
  (bind _rowbeingcached (`local.RowBeingCached`))
  (bind _value (`BlueprintMapLibrary.Map_Find` _cellsaliveatstart _rowbeingcached))
  (`BlueprintMapLibrary.Map_Clear` (`self.CellsAliveAtStart`))
  (for _array_element (`self.InitialNodes`)
    (bind (_name _cells _rootoffset) (break `/Game/Types/Structs/LifeShape` _array_element))
    (for _array_element_2 _cells
      (bind (_row _column) (break `/Game/Types/Structs/LifeCell` _rootoffset))
      (bind (_row_2 _column_2) (break `/Game/Types/Structs/LifeCell` _array_element_2))
      (set `local.RowBeingCached` (+ _row _row_2))
      (set `local.ColumnBeingCached` (+ _column_2 _column))
      (if (`BlueprintMapLibrary.Map_Contains` _cellsaliveatstart _rowbeingcached)
        (bind _output_get (set `local.Cells` (`.Cells_3_2736CB634A50A057C35302ADDD968B86` (break `/Game/Types/Structs/LifeShapeRow` _value))))
        (`KismetArrayLibrary.Array_Add` _output_get (`local.ColumnBeingCached`))
        (bind _structout (setmembers `/Game/Types/Structs/LifeShapeRow` :`StructRef` _value :`Cells` (`local.Cells`)))
        (`BlueprintMapLibrary.Map_Add` _cellsaliveatstart (`local.RowBeingCached`) _structout)
        (else
          (`BlueprintMapLibrary.Map_Add` _cellsaliveatstart _rowbeingcached (make `/Game/Types/Structs/LifeShapeRow` (`|MakeArray` (`local.ColumnBeingCached`)))))))))

(fn `PrepareTexture`
  (bind _returnvalue (* (`self.Padding`) 2))
  (bind _display (`/Game/Blueprints/SimpleScreen.Display` (`self.Screen`)))
  (bind _returnvalue_2 (`|GenericCreateObject` "/Script/game_of_life.DynamicTexture"))
  (bind _output_get (set `self.Texture` _returnvalue_2))
  (`DynamicTexture.Initialize` :`self` _output_get :`InWidth` (+ (`KismetMathLibrary.Max` (`self.Height`) 1) _returnvalue) :`InHeight` (+ (`KismetMathLibrary.Max` (`self.Width`) 1) _returnvalue) :`FilterMethod` "TF_Nearest")
  (bind _returnvalue_3 (`PrimitiveComponent.CreateDynamicMaterialInstance` _display 0 "/Game/Blueprints/LifeMaterial.LifeMaterial" "None"))
  (bind _output_get_2 (set `self.ScreenMaterial` _returnvalue_3))
  (`PrimitiveComponent.SetMaterial` _display 0 _output_get_2)
  (`self.UpdateScreen`))

(fn `UpdateScreen`
  (bind _padding (`self.Padding`))
  (for (_array_element _array_index) (`self.Rows`)
    (for (_array_element_2 _array_index_2) (`.Cells_2_D70D34C248750123A4A2D180AB2CE047` (break `/Game/Types/Structs/LifeRow` _array_element))
      (`DynamicTexture.SetPixel` (`self.Texture`) (+ _array_index _padding) (+ (- (`self.Width`) _array_index_2) _padding) (`KismetMathLibrary.SelectColor` (struct :`R` 1.0 :`G` 1.0 :`B` 1.0 :`A` 1.0) (struct) _array_element_2))))
  (`DynamicTexture.UpdateTexture` (`self.Texture`))
  (`MaterialInstanceDynamic.SetTextureParameterValue` (`self.ScreenMaterial`) "Texture" (`DynamicTexture.GetTextureResource` (`self.Texture`))))

(fn `UserConstructionScript`)