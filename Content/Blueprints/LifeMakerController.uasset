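; LifeMakerController is a player controller that drives a cellular Life simulation.
; On BeginPlay it caches the level's BP_Life actor, then forwards input actions to it for stepping an iteration, changing speed and resetting.
; Look and turn axes add pitch and yaw to the controlled pawn.
; The construction script fills Palette with index-named, filled square LifeShape brushes of increasing size, built procedurally from LifeCells.
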(event `self.ReceiveBeginPlay`
  (bind _returnvalue (`GameplayStatics.GetActorOfClass` "/Game/Blueprints/BP_Life.BP_Life_C"))
  (set `self.Life` _returnvalue))

(event `self.ReceivePossess`
  (params (PossessedPawn :type "Pawn Object Reference")))

(event `InputAxis|LookUp`
  (params (AxisValue :type "Float (single-precision)"))
  (`Pawn.AddControllerPitchInput` (`self.K2_GetPawn`) AxisValue))

(event `InputAxis|TurnRight`
  (params (AxisValue :type "Float (single-precision)"))
  (`Pawn.AddControllerYawInput` (`self.K2_GetPawn`) AxisValue))

(event `InputAction|Iterate`
  (params (Key :type "Key Structure"))
  (:`Pressed`
    (`/Game/Blueprints/BP_Life.LifeIteration` (`self.Life`))))

(event `InputAction|SpeedUp`
  (params (Key :type "Key Structure"))
  (:`Pressed`
    (`/Game/Blueprints/BP_Life.ChangeSpeed` (`self.Life`) true)))

(event `InputAction|SpeedDown`
  (params (Key :type "Key Structure"))
  (:`Pressed`
    (`/Game/Blueprints/BP_Life.ChangeSpeed` (`self.Life`) false)))

(event `InputAction|Reset`
  (params (Key :type "Key Structure"))
  (:`Pressed`
    (`Life.Reset` (`self.Life`))))

(fn `GenerateBrushes`
  (locals (CurrentBrushCells :type "Array of /Game/Types/Structs/LifeCell Structure"))
  (`KismetArrayLibrary.Array_Clear` (`self.Palette`))
  (for _index (range 10)
    (`KismetArrayLibrary.Array_Clear` (`local.CurrentBrushCells`))
    (for _index_2 (range (+ _index 1))
      (for _index_3 (range (+ _index 1))
        (`KismetArrayLibrary.Array_Add` (`local.CurrentBrushCells`) (make `/Game/Types/Structs/LifeCell` _index_2 _index_3))))
    (`KismetArrayLibrary.Array_Add` (`self.Palette`) (make `/Game/Types/Structs/LifeShape` (`KismetStringLibrary.Conv_IntToString` _index) (`local.CurrentBrushCells`)))))

(fn `UserConstructionScript`
  (`self.GenerateBrushes`))