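; LifeGameMode is a game mode Blueprint that runs a random-value loop test on BeginPlay and prints the results.
; A while loop increments a counter and calls Loopbody until Bingo is true, then prints a completion message.
; Loopbody randomizes bool, int and float values, sets Bingo when the bool and int threshold both pass, and prints all values when either passes.
; An unconnected for-loop alternative remains in the graph.
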(event `self.ReceiveBeginPlay`
  (bind _boolvar (`self.boolvar`))
  (while (not (`self.Bingo`))
    (set `self.loopIndex` (+ (`self.loopIndex`) 1))
    (set `self.boolvar` (`KismetMathLibrary.RandomBool`))
    (bind _output_get (set `self.intvar` (`KismetMathLibrary.RandomIntegerInRange` 100 1000)))
    (set `self.floatvar` (`KismetMathLibrary.RandomFloatInRange` 1.0 15.0))
    (set `self.stingvar` (`KismetSystemLibrary.GetDisplayName` self))
    (bind _returnvalue (> _output_get 500))
    (set `self.Bingo` (and _returnvalue _boolvar))
    (if (or _boolvar _returnvalue)
      (`KismetSystemLibrary.PrintString` (`KismetStringLibrary.Concat_StrStr` (`KismetStringLibrary.Conv_IntToString` (`self.loopIndex`)) " | int: " (`KismetStringLibrary.Conv_IntToString` (`self.intvar`)) " | float: " (`KismetStringLibrary.Conv_DoubleToString` (`self.floatvar`)) " | string: " (`self.stingvar`) " | bool: " (`KismetStringLibrary.Conv_BoolToString` (`self.boolvar`))) true true (struct :`R` 0.213542 :`G` 1.0 :`B` 0.246637 :`A` 1.0) 10.0)))
  (`KismetSystemLibrary.PrintString` "Вone"))

(fn `UserConstructionScript`)